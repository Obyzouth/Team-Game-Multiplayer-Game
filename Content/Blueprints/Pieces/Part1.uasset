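; Part1 is a collectible part actor that picks a random visual variation when it spawns.
; On BeginPlay, a random integer toggles the visibility of one of ten numbered components, though a roll of 10 matches no case.
; PartPickedUp destroys the actor and returns a count of one, ignoring its Count input.
; Destroyonserver destroys the particle system and numbered components, then the actor.
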(event Custom|Destroy%20on%20server
  (Components|DestroyComponent (Variables|Default|GetParticleSystem))
  (Actor|DestroyActor))

(event EventBeginPlay
  (switch int (Math|Random|RandomIntegerinRange 0 10)
    (:0
      (Rendering|ToggleVisibility (Variables|Default|Get1) false))
    (:1
      (Rendering|ToggleVisibility (Variables|Default|Get2) false))
    (:2
      (Rendering|ToggleVisibility (Variables|Default|Get3) false))
    (:3
      (Rendering|ToggleVisibility (Variables|Default|Get4) false))
    (:4
      (Rendering|ToggleVisibility (Variables|Default|Get5) false))
    (:5
      (Rendering|ToggleVisibility (Variables|Default|Get6) false))
    (:6
      (Rendering|ToggleVisibility (Variables|Default|Get7) false))
    (:7
      (Rendering|ToggleVisibility (Variables|Default|Get8) false))
    (:8
      (Rendering|ToggleVisibility (Variables|Default|Get9) false))
    (:9
      (Rendering|ToggleVisibility (Variables|Default|Get10) false))))

(event Collision|EventActorBeginOverlap
  (params (OtherActor :type Actor%20Object%20Reference)))

(event EventTick
  (params (DeltaSeconds :type Float%20%28single-precision%29)))

(event Collision|EventHit
  (params (MyComp :type Primitive%20Component%20Object%20Reference) (Other :type Actor%20Object%20Reference) (OtherComp :type Primitive%20Component%20Object%20Reference) (bSelfMoved :type Boolean) (HitLocation :type Vector :default "0, 0, 0") (HitNormal :type Vector :default "0, 0, 0") (NormalImpulse :type Vector :default "0, 0, 0") (Hit :type Hit%20Result%20Structure%20%28by%20ref%29)))

(fn ConstructionScript)

(fn PartPickedUp
  (params (Count :type Integer))
  (Actor|DestroyActor)
  (return (+ 0 1)))